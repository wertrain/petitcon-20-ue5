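; HelixPropel game state that tracks the current level number and looks up its definition.
; GetCurrentGameLevel scans the rows of DT_GameLevel and returns the one whose Level matches CurrentLevel.
; SetGameLevel stores a new level and fires the OnLevelChanged dispatcher, while IncrementLevel bumps the value without broadcasting.
; BeginPlay and Tick are empty.
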(fn `GetCurrentGameLevel`
  (returns (`Out GameLevel` :type "/Game/HelixPropel/GameData/ST_GameLevel Structure"))
  (bind _outrownames (`DataTableFunctionLibrary.GetDataTableRowNames` "/Game/HelixPropel/GameData/DT_GameLevel.DT_GameLevel"))
  (for _array_element _outrownames
    (bind _returnvalue (`|GetDataTableRow` "/Game/HelixPropel/GameData/DT_GameLevel.DT_GameLevel" _array_element)
      (:`then`
        (if (== (`self.CurrentLevel`) (`.Level_2_69DA5769418E0D2322AC58B8D8C9DC1E` (break `/Game/HelixPropel/GameData/ST_GameLevel` _returnvalue)))
          (return _returnvalue))))))

(fn `IncrementLevel`
  (returns (`Out Level` :type Integer))
  (bind _result (`/Engine/EditorBlueprintResources/StandardMacros.IncrementInt` (`self.CurrentLevel`))
    (:`  `
      (return _result))))

(fn `SetGameLevel`
  (params (`In Level` :type Integer))
  (bind _output_get (set `self.CurrentLevel` `In Level`))
  (`self.OnLevelChanged` _output_get))

(fn `UserConstructionScript`)