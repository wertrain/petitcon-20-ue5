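; Player state for HelixPropel that tracks the player's score and combo count.
; Combo functions add to or reset the count and broadcast each change through OnComboCountChanged.
; CalculateComboBonusScore adds the incoming score plus a rounded bonus scaled by the natural log of the combo, broadcasts OnScoreChanged and returns the new total.
; Begin Play, Tick and the construction script are empty.
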(fn `AddComboCount`
  (params (`In Count` :type Integer))
  (bind _output_get (set `self.ComboCount` (+ `In Count` (`self.ComboCount`))))
  (`self.OnComboCountChanged` _output_get))

(fn `CalculateComboBonusScore`
  (params (`In Score` :type Integer))
  (returns (`Out Score` :type Integer))
  (bind _output_get (set `self.PlayerScore` (+ (`self.PlayerScore`) (+ (`KismetMathLibrary.Round` (* `In Score` (`KismetMathLibrary.Loge` (`KismetMathLibrary.Conv_IntToDouble` (`self.ComboCount`))))) (`local.In Score`)))))
  (`self.OnScoreChanged` _output_get)
  (return _output_get))

(fn `ResetCombo`
  (bind _output_get (set `self.ComboCount` 0))
  (`self.OnComboCountChanged` _output_get))

(fn `UserConstructionScript`)