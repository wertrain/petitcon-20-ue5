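; BP_Player is the player actor in HelixPropel, propelled along the world X axis.
; Tick adds Acceleration to PropelPower each frame, then applies a delta-time-scaled, unswept offset.
; ReverseMovement flips positive power into a clamped negative kick with a guaranteed minimum strength.
; Bounce flips it with damping, disabling tick and returning true once the rebound is too weak.
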(event `self.ReceiveTick`
  (params (DeltaSeconds :type "Float (single-precision)"))
  (bind _output_get (set `self.PropelPower` (+ (`self.PropelPower`) (`self.Acceleration`))))
  (`self.K2_AddActorWorldOffset` (`KismetMathLibrary.MakeVector` (* _output_get DeltaSeconds))))

(fn `Bounce`
  (returns (bEndBounce :type Boolean))
  (if (> (`self.PropelPower`) 0.0)
    (bind _output_get (set `self.PropelPower` (`KismetMathLibrary.FClamp` (* (* (`self.PropelPower`) 0.8) -1.0) (* (`self.Acceleration`) -20.0) 0.0)))
    (if (< _output_get -200.0)
      (return false)
      (else
        (`self.SetActorTickEnabled` false)
        (return true)))))

(fn `ReverseMovement`
  (if (> (`self.PropelPower`) 0.0)
    (set `self.PropelPower` (`KismetMathLibrary.FClamp` (* (`self.PropelPower`) -1.0) (* (`self.Acceleration`) -30.0) -1000.0))))

(fn `UserConstructionScript`)