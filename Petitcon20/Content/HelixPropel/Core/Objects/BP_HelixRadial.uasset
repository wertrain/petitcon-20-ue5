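; BP_HelixRadial is one ring of a helix level, built on BeginPlay from BP_HelixUnit segments with random gaps and randomly assigned damage types.
; It shuffles sixteen slot indices, removes a random number, and spawns units for the rest.
; Pawn overlaps confirmed by the unit's IsHit broadcast its type as an unbreakable hit, while Box overlaps broadcast a breakable hit.
; OffsetAngle turns all units; Collapse enables their physics and disables the Box.
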(event `self.ReceiveBeginPlay`
  (bind _size (`self.RadialSize`))
  (`|ExecutionSequence`
    (:`then_0`
      ;[1 1 1] ランダムに欠けたインデックス配列を作成
      (for _index (range 16)
        (`KismetArrayLibrary.Array_Add` (`self.Indices`) _index))
      (`KismetArrayLibrary.Array_Shuffle` (`self.Indices`))
      (for _index_2 (range (+ (`KismetMathLibrary.RandomIntegerInRange` (`self.UnitRemoveRangeMin`) (`self.UnitRemoveRangeMax`)) 1))
        (`KismetArrayLibrary.Array_Remove` (`self.Indices`) _index_2)))
    (:`then_1`
      ;[1 1 1] 作成したインデックス配列を元に Helix Unit を並べる
      (for _array_element (`self.Indices`)
        (bind _returnvalue (`|SpawnActorFromClass` "/Game/HelixPropel/Core/Objects/BP_HelixUnit.BP_HelixUnit_C" (`KismetMathLibrary.MakeTransform` (`self.K2_GetActorLocation`) (struct) (`KismetMathLibrary.MakeVector` _size _size 10.0)) "Undefined" "OverrideRootScale" null _array_element null))
        (`KismetArrayLibrary.Array_Add` (`self.Units`) _returnvalue)
        (add `PrimitiveComponent.OnComponentBeginOverlap` (`/Game/HelixPropel/Core/Objects/BP_HelixUnit.NearRadialCollision` _returnvalue) (delegate `OnOverlapRadialCheckArea`))))
    (:`then_2`
      (for _array_element_2 (`self.Units`)
        (if (`KismetMathLibrary.RandomBoolWithWeight` (`self.DamageUnitRate`))
          (`/Game/HelixPropel/Core/Objects/BP_HelixUnit.SetType` _array_element_2 "NewEnumerator1"))))))

(event `OnOverlapRadialCheckArea`
  (params (OverlappedComponent :type "PrimitiveComponent Object Reference") (OtherActor :type "Actor Object Reference") (OtherComp :type "PrimitiveComponent Object Reference") (OtherBodyIndex :type Integer) (bFromSweep :type Boolean) (SweepResult :type "HitResult Structure (by ref)"))
  (bind _aspawn (cast `Pawn` OtherActor))
  (bind _asbp_helix_unit (cast `/Game/HelixPropel/Core/Objects/BP_HelixUnit` (`ActorComponent.GetOwner` OverlappedComponent)))
  (bind _out_result (`/Game/HelixPropel/Core/Objects/BP_HelixUnit.IsHit` _asbp_helix_unit (`self.K2_GetActorLocation` _aspawn) 0.0))
  (if _out_result
    (`self.OnHitUnbreakableArea` (`/Game/HelixPropel/Core/Objects/BP_HelixUnit.Type` _asbp_helix_unit))))

(event `self.Box.OnComponentBeginOverlap`
  (params (OverlappedComponent :type "PrimitiveComponent Object Reference") (OtherActor :type "Actor Object Reference") (OtherComp :type "PrimitiveComponent Object Reference") (OtherBodyIndex :type Integer) (bFromSweep :type Boolean) (SweepResult :type "HitResult Structure (by ref)"))
  (`self.OnHitBreakableArea` self))

(fn `Collapse`
  (`self.SetSimulatePhysics` true)
  (`PrimitiveComponent.SetCollisionEnabled` (`self.Box`) "NoCollision"))

(fn `OffsetAngle`
  (params (`In Angle` :type "Float (double-precision)"))
  (for _array_element (`self.Units`)
    (`/Game/HelixPropel/Core/Objects/BP_HelixUnit.OffsetAngle` _array_element `In Angle`)))

(fn `SetSimulatePhysics`
  (params (bSimulate :type Boolean))
  (for _array_element (`self.Units`)
    (`PrimitiveComponent.SetSimulatePhysics` (`/Game/HelixPropel/Core/Objects/BP_HelixUnit.StaticMesh` _array_element) bSimulate)))

(fn `UserConstructionScript`)