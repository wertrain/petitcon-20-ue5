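; BP_RouteMover is a prototype actor that propels itself along world X and destroys itself on any hit.
; Each Tick adds Acceleration to PropelPower without delta-time scaling, then applies a delta-scaled, non-swept offset.
; ReverseMovement flips positive power to negative, clamped to a band derived from Acceleration, whose graph is empty here.
; SetSimulatePhysics toggles physics on the Sphere component.
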(event `self.ReceiveTick`
  (params (DeltaSeconds :type "Float (single-precision)"))
  (bind _output_get (set `self.PropelPower` (+ (`self.PropelPower`) (`self.Acceleration`))))
  (`self.K2_AddActorWorldOffset` (`KismetMathLibrary.MakeVector` (* _output_get DeltaSeconds))))

(event `self.Sphere.OnComponentHit`
  (params (HitComponent :type "PrimitiveComponent Object Reference") (OtherActor :type "Actor Object Reference") (OtherComp :type "PrimitiveComponent Object Reference") (NormalImpulse :type "Vector Structure") (Hit :type "HitResult Structure (by ref)"))
  (`self.K2_DestroyActor` :!label _label))

(event `self.ReceiveHit`
  (params (MyComp :type "PrimitiveComponent Object Reference") (Other :type "Actor Object Reference") (OtherComp :type "PrimitiveComponent Object Reference") (bSelfMoved :type Boolean) (HitLocation :type "Vector Structure") (HitNormal :type "Vector Structure") (NormalImpulse :type "Vector Structure") (Hit :type "HitResult Structure (by ref)"))
  (goto _label))

(event `self.Collision.OnComponentHit`
  (params (HitComponent :type "PrimitiveComponent Object Reference") (OtherActor :type "Actor Object Reference") (OtherComp :type "PrimitiveComponent Object Reference") (NormalImpulse :type "Vector Structure") (Hit :type "HitResult Structure (by ref)"))
  (goto _label))

(fn `ReverseMovement`
  (if (> (`self.PropelPower`) 0.0)
    (set `self.PropelPower` (`KismetMathLibrary.FClamp` (* (`self.PropelPower`) -1.0) (* (`self.Acceleration`) -50.0) (* (`self.Acceleration`) -40.0)))))

(fn `Set Simulate Physics`
  (params (bSimulate :type Boolean))
  (`PrimitiveComponent.SetSimulatePhysics` (`self.Sphere`) bSimulate))

(fn `UserConstructionScript`)